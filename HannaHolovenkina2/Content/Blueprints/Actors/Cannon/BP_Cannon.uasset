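; Automatic cannon actor that repeatedly fires BP_Bullet from BeginPlay, after a Firerate delay.
; Each bullet spawns at the Arrow component's world location and rotation, sized by Scale.
; The Shooting timeline then restarts to animate Cannon recoil along relative Y.
; Its Update output feeds back into the Delay, so the timeline itself keeps the firing loop running.
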(event EventBeginPlay
  (bind _arrow (Variables|Default|GetArrow))
  (Utilities|FlowControl|Delay (Variables|CannonProperties|GetFirerate) :!label _label)
  (Game|SpawnActorfromClass "/Game/Blueprints/Actors/Projectiles/BP_Bullet.BP_Bullet_C" (Math|Transform|MakeTransform (Transformation|GetWorldLocation _arrow) (Transformation|GetWorldRotation _arrow) (Math|Conversions|ToVector(Float) (Variables|CannonProperties|GetScale))) "Undefined" 0 0)
  (bind _cannonrecoil (Timeline|Shooting PlayFromStart)
    (:Update
      (Transformation|SetRelativeLocation (Variables|Default|GetCannon) (Math|Vector|MakeVector 0.0 _cannonrecoil 0.0) false false)
      (goto _label))))

(fn ConstructionScript)