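; BP_Crystal is a collectable crystal that reacts to the player overlapping its sphere, but shows no reward logic.
; On overlap it caches its location and light intensity, then plays the CrystalTransform timeline.
; The timeline's curves pull it toward the player's live position, shrink it and fade its point light before it destroys itself.
; Scale lerps from the current value each update, so shrinking compounds.
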(event OnComponentBeginOverlap(Sphere)
  (params (OverlappedComponent :type Primitive%20Component%20Object%20Reference) (OtherActor :type Actor%20Object%20Reference) (OtherComp :type Primitive%20Component%20Object%20Reference) (OtherBodyIndex :type Integer) (bFromSweep :type Boolean) (SweepResult :type Hit%20Result%20Structure%20%28by%20ref%29))
  (Utilities|IsPlayer OtherActor)
  (CallFunction|Varibles)
  (bind (_direction _location _scale _light) (Timeline|Crystal%20transform Play)
    (:Update
      (CallFunction|Location _location)
      (CallFunction|Scale _scale)
      (CallFunction|Intencity _light))
    (:Finished
      (Actor|DestroyActor))))

(fn ConstructionScript)

(fn Location
  (params (Alpha :type Float%20%28single-precision%29))
  (Transformation|SetActorLocation (Math|Vector|Lerp(Vector) (Variables|Default|GetLerpStartLocation) (Transformation|GetActorLocation (Game|Player|GetPlayerPawn 0)) Alpha) false false))

(fn Scale
  (params (Alpha :type Float%20%28single-precision%29))
  (Transformation|SetActorScale3D (Math|Vector|Lerp(Vector) (Transformation|GetActorScale3D) "0, 0, 0" Alpha)))

(fn Intencity
  (params (Alpha :type Float%20%28single-precision%29))
  (Rendering|Components|Light|SetIntensity (Variables|Default|GetPointLight) (Math|Float|Lerp (Variables|Default|GetLightIntensity) 0.0 Alpha)))

(fn Varibles
  (Variables|Default|SetLerpStartLocation (Transformation|GetActorLocation))
  (Variables|Default|SetLightIntensity (Variables|/Script/Engine.LightComponentBase|GetIntensity (Variables|Default|GetPointLight))))