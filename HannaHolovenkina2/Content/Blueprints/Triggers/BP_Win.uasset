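; BP_Win is a level exit trigger that completes the level when its Box is overlapped and no BP_Crystal actors remain.
; With crystals left, it prints a debug string and reloads the current level after a delay.
; Completion looks up the current level in the LevelName array and quits on the last entry.
; Otherwise NextLevel increments that index but opens the array's first entry, not the incremented one.
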(event OnComponentBeginOverlap(Box)
  (params (OverlappedComponent :type Primitive%20Component%20Object%20Reference) (OtherActor :type Actor%20Object%20Reference) (OtherComp :type Primitive%20Component%20Object%20Reference) (OtherBodyIndex :type Integer) (bFromSweep :type Boolean) (SweepResult :type Hit%20Result%20Structure%20%28by%20ref%29))
  (if (CallFunction|CheckAnyCrystals)
    (Development|PrintString "Hello")
    (Utilities|FlowControl|Delay 2.0)
    (bind _returnvalue (Game|GetCurrentLevelName true))
    (Game|OpenLevel(byName) (Utilities|String|StringToName _returnvalue))
    (else
      (CallFunction|CompleteLevel))))

(fn ConstructionScript)

(fn CheckAnyCrystals
  (bind _outactors (Actor|GetAllActorsOfClass "/Game/Blueprints/Actors/Collectables/BP_Crystal.BP_Crystal_C"))
  (return (> (Utilities|Array|Length _outactors) 0)))

(fn CompleteLevel
  (if (CallFunction|IsFinal)
    (Game|QuitGame 0 "Quit" false)
    (else
      (CallFunction|NextLevel))))

(fn NextLevel
  (Math|Integer|IncrementInt (CallFunction|LevelIndex)
    (:%20%20
      (Game|OpenLevel(byName) (Utilities|Array|Get(acopy) (Variables|Default|GetLevelName))))))

(fn LevelIndex
  (bind _returnvalue (Game|GetCurrentLevelName true))
  (return (Utilities|Array|FindItem (Variables|Default|GetLevelName) (Utilities|String|StringToName _returnvalue))))

(fn IsFinal
  (return (== (Utilities|Array|LastIndex (Variables|Default|GetLevelName)) (CallFunction|LevelIndex))))